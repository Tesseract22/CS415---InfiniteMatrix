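; Endless-runner tunnel segment with a rotating holed wall, a bobbing health pack and an enemy that a bullet can destroy.
; Exposes functions to randomize the wall, randomly remove or offset both components, and tint the dynamic material red-to-green by health percent.
; Wall and enemy hits cost player HP; the pack restores it.
; The exit trigger has TunnelSpawner spawn another tunnel, destroys this one, and awards score and speed if the wall was avoided.
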(event OnComponentBeginOverlap(TriggerZone)
  (params (OverlappedComponent :type Primitive%20Component%20Object%20Reference) (OtherActor :type Actor%20Object%20Reference) (OtherComp :type Primitive%20Component%20Object%20Reference) (OtherBodyIndex :type Integer) (bFromSweep :type Boolean) (SweepResult :type Hit%20Result%20Structure%20%28by%20ref%29))
  (bind _asbp_player (Utilities|Casting|CastToBP_Player OtherActor))
  (Default|SpawnTunnelatSpawnPoint (Variables|Default|GetTunnelSpawner))
  (Actor|DestroyActor)
  (if (not (Variables|Default|GetCollided))
    (Default|AddScore _asbp_player)
    (Variables|/Game/InfiniteMatrix/Blueprints/BP_Player.BP_Player_C|SetFowardSpeed _asbp_player (+ (Variables|/Game/InfiniteMatrix/Blueprints/BP_Player.BP_Player_C|GetFowardSpeed _asbp_player) 1e+02))))

(event OnComponentBeginOverlap(WallMesh)
  (params (OverlappedComponent :type Primitive%20Component%20Object%20Reference) (OtherActor :type Actor%20Object%20Reference) (OtherComp :type Primitive%20Component%20Object%20Reference) (OtherBodyIndex :type Integer) (bFromSweep :type Boolean) (SweepResult :type Hit%20Result%20Structure%20%28by%20ref%29))
  (bind _asbp_player (Utilities|Casting|CastToBP_Player OtherActor)
    (:then
      (Default|ReduceHp _asbp_player)
      (Variables|Default|SetCollided true))
    (:CastFailed
      (bind _asbp_bullet (Utilities|Casting|CastToBP_Bullet OtherActor))
      (Actor|DestroyActor _asbp_bullet))))

(event OnComponentBeginOverlap(HealthPack)
  (params (OverlappedComponent :type Primitive%20Component%20Object%20Reference) (OtherActor :type Actor%20Object%20Reference) (OtherComp :type Primitive%20Component%20Object%20Reference) (OtherBodyIndex :type Integer) (bFromSweep :type Boolean) (SweepResult :type Hit%20Result%20Structure%20%28by%20ref%29))
  (bind _asbp_player (Utilities|Casting|CastToBP_Player OtherActor))
  (Default|AddHp _asbp_player)
  (Components|DestroyComponent (Variables|Default|GetHealthPack)))

(event OnComponentBeginOverlap(Enemy)
  (params (OverlappedComponent :type Primitive%20Component%20Object%20Reference) (OtherActor :type Actor%20Object%20Reference) (OtherComp :type Primitive%20Component%20Object%20Reference) (OtherBodyIndex :type Integer) (bFromSweep :type Boolean) (SweepResult :type Hit%20Result%20Structure%20%28by%20ref%29))
  (bind _asbp_player (Utilities|Casting|CastToBP_Player OtherActor)
    (:then
      (Default|ReduceHp _asbp_player))
    (:CastFailed
      (bind _asbp_bullet (Utilities|Casting|CastToBP_Bullet OtherActor))
      (Actor|DestroyActor _asbp_bullet)))
  (Components|DestroyComponent (Variables|Default|GetEnemy)))

(event EventBeginPlay)

(event EventTick
  (params (DeltaSeconds :type Float%20%28single-precision%29))
  (Utilities|FlowControl|Sequence
    (:then_0
      (Variables|Default|Settime (+ (Variables|Default|Gettime) DeltaSeconds)))
    (:then_1
      (Transformation|AddLocalRotation (Variables|Default|GetWallMesh) (Math|Rotator|MakeRotator (* DeltaSeconds (Variables|Default|GetRotateSpeed)) 0.0 0.0) false false)
      (CallFunction|Floating))))

(fn ConstructionScript
  (bind _returnvalue (Rendering|Material|CreateDynamicMaterialInstance (Variables|Debug|GetStaticMeshComponent) 0 "/Game/InfiniteMatrix/Materials/MI_Tunnel.MI_Tunnel" "None" :!class /Script/Engine.PrimitiveComponent))
  (Variables|Default|SetTunnelMaterial _returnvalue))

(fn RandomizedWall
  (Components|StaticMesh|SetStaticMesh (Variables|Default|GetWallMesh) (Utilities|Select :Index (Math|Random|RandomIntegerinRange 0 3) :Option%200 "/Game/InfiniteMatrix/Meshes/SM_Hole_01.SM_Hole_01" :Option%201 "/Game/InfiniteMatrix/Meshes/SM_Hole_02.SM_Hole_02" :Option%202 "/Game/InfiniteMatrix/Meshes/SM_Hole_03.SM_Hole_03" :Option%203 "/Game/InfiniteMatrix/Meshes/SM_Hole_04.SM_Hole_04"))
  (Transformation|AddLocalRotation (Variables|Default|GetWallMesh) (Math|Rotator|MakeRotator (Math|Random|RandomFloatinRange 0.0 3.6e+02) 0.0 0.0) false false))

(fn RandomizedHealthPack
  (bind _healthpack (Variables|Default|GetHealthPack))
  (if (Math|Random|RandomBool)
    (Components|DestroyComponent _healthpack)
    (else
      (Transformation|AddLocalOffset _healthpack (Math|Vector|MakeVector (Math|Random|RandomFloatinRange -1e+03 1e+03) (Math|Random|RandomFloatinRange -3e+02 3e+02) (Math|Random|RandomFloatinRange -3e+02 3e+02)) false true))))

(fn RandomizedEnemy
  (bind _enemy (Variables|Default|GetEnemy))
  (if (Math|Random|RandomBool)
    (Components|DestroyComponent _enemy)
    (else
      (Transformation|AddLocalOffset _enemy (Math|Vector|MakeVector (Math|Random|RandomFloatinRange -1e+03 1e+03) (Math|Random|RandomFloatinRange -3e+02 3e+02) (Math|Random|RandomFloatinRange -3e+02 3e+02)) false true))))

(fn Floating
  (bind _healthpack (Variables|Default|GetHealthPack))
  (if (Utilities|IsValid _healthpack)
    (Transformation|AddLocalOffset _healthpack (Math|Vector|MakeVector 0.0 0.0 (* 1.5 (Math|Trig|Sin(Degrees) (* (Variables|Default|Gettime) 1e+02)))) true false)))

(fn ChangeColor
  (params (HealthPercent :type Float%20%28double-precision%29))
  (Rendering|Material|SetVectorParameterValue (Variables|Default|GetTunnelMaterial) "BackgroundColor" (Class|KismetMathLibrary|LinearColorLerpUsingHSV (Class|KismetMathLibrary|LinearColorRed) (Class|KismetMathLibrary|LinearColorGreen) HealthPercent) :!class /Script/Engine.MaterialInstanceDynamic))