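; BP_Bullet is a projectile actor that travels along world X at a speed tied to the player's forward speed.
; Each tick it casts the player pawn to BP_Player and moves by a swept world offset at triple that FowardSpeed, scaled by delta time.
; It accumulates elapsed time and destroys itself after a very long lifetime threshold; it contains no hit or damage logic.
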(event EventBeginPlay)

(event Collision|EventActorBeginOverlap
  (params (OtherActor :type Actor%20Object%20Reference)))

(event EventTick
  (params (DeltaSeconds :type Float%20%28single-precision%29))
  (bind _asbp_player (Utilities|Casting|CastToBP_Player (Game|Player|GetPlayerPawn 0)))
  (Transformation|AddActorWorldOffset (Math|Vector|MakeVector (* (Variables|/Game/InfiniteMatrix/Blueprints/BP_Player.BP_Player_C|GetFowardSpeed _asbp_player) DeltaSeconds 3.0) 0.0 0.0) true)
  (bind _output_get (Variables|Default|SetTimePast (+ DeltaSeconds (Variables|Default|GetTimePast))))
  (if (> _output_get 1e+03)
    (Actor|DestroyActor)))

(fn ConstructionScript)